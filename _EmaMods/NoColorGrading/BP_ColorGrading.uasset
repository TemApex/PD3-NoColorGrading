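; Mod actor that removes color grading from heist levels when play begins.
; It sets the LUT intensity to zero on every PostProcessVolume in the level.
; For the branch bank heist (NRFTW), it also turns the first SkyLight white.
; That heist is detected by comparing the mission state's display name to a string table entry, so the check follows any official rename.
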(event `self.ReceiveBeginPlay`
  ;[1 1 1] Every other heist
  (bind _outactors (`GameplayStatics.GetAllActorsOfClass` "/Script/Engine.PostProcessVolume"))
  (for _array_element _outactors
    (bind _output_get (set `self.PP` _array_element))
    (setmembers `PostProcessSettings` :`StructRef` (`PostProcessVolume.Settings` _output_get) :`TemperatureType` "TEMP_WhiteBalance" :`WhiteTemp` 6500.0 :`WhiteTint` 0.0 :`ColorSaturation` (1.0 1.0 1.0 1.0) :`ColorContrast` (1.0 1.0 1.0 1.0) :`ColorGamma` (1.0 1.0 1.0 1.0) :`ColorGain` (1.0 1.0 1.0 1.0) :`ColorOffset` (0.0 0.0 0.0 0.0) :`ColorSaturationShadows` (1.0 1.0 1.0 1.0) :`ColorContrastShadows` (1.0 1.0 1.0 1.0) :`ColorGammaShadows` (1.0 1.0 1.0 1.0) :`ColorGainShadows` (1.0 1.0 1.0 1.0) :`ColorOffsetShadows` (0.0 0.0 0.0 0.0) :`ColorSaturationMidtones` (1.0 1.0 1.0 1.0) :`ColorContrastMidtones` (1.0 1.0 1.0 1.0) :`ColorGammaMidtones` (1.0 1.0 1.0 1.0) :`ColorGainMidtones` (1.0 1.0 1.0 1.0) :`ColorOffsetMidtones` (0.0 0.0 0.0 0.0) :`ColorSaturationHighlights` (1.0 1.0 1.0 1.0) :`ColorContrastHighlights` (1.0 1.0 1.0 1.0) :`ColorGammaHighlights` (1.0 1.0 1.0 1.0) :`ColorGainHighlights` (1.0 1.0 1.0 1.0) :`ColorOffsetHighlights` (0.0 0.0 0.0 0.0) :`ColorCorrectionHighlightsMin` 0.5 :`ColorCorrectionShadowsMax` 0.09 :`BlueCorrection` 0.6 :`ExpandGamut` 1.0 :`ToneCurveAmount` 1.0 :`SceneColorTint` (struct :`R` 1.0 :`G` 1.0 :`B` 1.0 :`A` 1.0) :`ColorGradingIntensity` 0.0))
  (if (`KismetTextLibrary.EqualEqual_TextText` (`PD3HeistDataAsset.HeistDisplayName` (`SBZMissionState.CurrentHeistData` (`SBZMissionState.GetSBZMissionState`))) "LVL_BB_HEISTNAME")
    ;[1 1 1] NRFTW Specific stuff
    (bind _outactors_2 (`GameplayStatics.GetAllActorsOfClass` "/Script/Engine.SkyLight"))
    (`SkyLightComponent.SetLightColor` (`SkyLight.LightComponent` (`|GetArrayItem` _outactors_2)) (struct :`R` 1.0 :`G` 1.0 :`B` 1.0 :`A` 1.0))))

(fn `UserConstructionScript`
  (`parent.UserConstructionScript`))